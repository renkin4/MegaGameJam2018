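; BP_PatrolPath is a patrol route actor with start and end arrow points that one AI officer at a time walks between.
; Officers claim the path through a try-to-patrol check that succeeds when it is free or already theirs, and release it on leaving.
; The next patrol point is an arrow's world location chosen by a destination index, which toggles whenever a patrol leg completes.
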(event EventBeginPlay)

(event Collision|EventActorBeginOverlap
  (params (OtherActor :type Actor%20Object%20Reference)))

(event EventTick
  (params (DeltaSeconds :type Float%20%28single-precision%29)))

(fn ConstructionScript)

(fn CanPatrol
  (params (NewOfficer :type BP%20AI%20Character%20Object%20Reference))
  (bind _activeofficer (Variables|Default|GetActiveOfficer))
  (return (or (== NewOfficer _activeofficer) (== _activeofficer 0))))

(fn TrytoPartrol
  (params (NewOfficer :type BP%20AI%20Character%20Object%20Reference))
  (if (CallFunction|CanPatrol NewOfficer)
    (Variables|Default|SetActiveOfficer NewOfficer)
    (return true)
    (else
      (return false))))

(fn TryLeavePatrol
  (params (LeavingOfficer :type BP%20AI%20Character%20Object%20Reference))
  (if (== (Variables|Default|GetActiveOfficer) LeavingOfficer)
    (Variables|Default|SetActiveOfficer 0))
  (return))

(fn GetNextPatrolPoint
  (return (Transformation|GetWorldLocation (Utilities|Select :Index (Variables|Default|GetDestinationIndex) :Option%200 (Variables|Default|GetArrow_End) :Option%201 (Variables|Default|GetArrow_Start)))))

(fn OnPatrolCompleted
  (Variables|Default|SetDestinationIndex (Utilities|Select :Index (Variables|Default|GetDestinationIndex) :Option%200 1 :Option%201 0)))