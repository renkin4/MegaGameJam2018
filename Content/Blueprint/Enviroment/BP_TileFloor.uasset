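; BP_TileFloor is an environment actor that builds a rectangular floor from a repeated mesh tile.
; Its construction script loops over the X and Y tile counts and adds an instance to the Floor1 instanced mesh component at each grid cell.
; Cell offsets come from the mesh width and length variables, with no rotation or scaling.
; The event graph has no active logic.
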(event EventBeginPlay)

(event Collision|EventActorBeginOverlap
  (params (OtherActor :type Actor%20Object%20Reference)))

(event EventTick
  (params (DeltaSeconds :type Float%20%28single-precision%29)))

(fn ConstructionScript
  (for _index (range 0 (- (Variables|Default|GetNumberMeshesX) 1))
    (for _index_2 (range 0 (- (Variables|Default|GetNumberMeshesY) 1))
      (Components|InstancedStaticMesh|AddInstance (Variables|Default|GetFloor_1) (Math|Transform|MakeTransform (Math|Vector|MakeVector (* _index (Variables|Default|GetMeshWidth)) (* _index_2 (Variables|Default|GetMeshLength)) 0.0))))))