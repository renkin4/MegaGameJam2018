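; BP_InventorySlot is an inventory slot that holds a single Inventory reference and counts as valid while that reference is valid.
; Setting the inventory stores it and passes the slot's CharacterOwner to it as pawn owner.
; Two use events forward to the held object's UseItem and UseItem2 after a validity check.
; Select and deselect events broadcast their matching delegates.
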(event Custom|UseItem
  ;[1 1 1] Use Item
  (bind _inventory (Variables|Default|GetInventory)
    (:then
      (Default|UseItem _inventory))
    (:else)))

(event Custom|OnSelected
  ;[1 1 1] Selection
  (Default|CallOnSelectedDelegate))

(event Custom|OnDeSelect
  ;[1 1 1] Selection
  (Default|CallOnDeSelectedDelegate))

(event Custom|SetInventory
  (params (NewInventory :type BP%20Inventory%20Item%20Base%20Object%20Reference))
  ;[1 1 1] Set Inventory
  (Variables|Default|SetInventory NewInventory)
  (Default|SetPawnOwner (Variables|Default|GetInventory) (Variables|Default|GetCharacterOwner)))

(event Custom|UseItem2
  ;[1 1 1] Use Item
  (bind _inventory (Variables|Default|GetInventory)
    (:then
      (Default|UseItem2 _inventory))
    (:else)))

(fn ConstructionScript)

(fn IsValidSlot
  (return (Utilities|IsValid (Variables|Default|GetInventory))))