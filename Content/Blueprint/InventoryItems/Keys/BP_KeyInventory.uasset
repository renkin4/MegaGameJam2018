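; Key inventory item that its owning character uses to open doors and cannot drop.
; Using it runs a short Visibility line trace from the character's location along its forward vector and sends a TryOpenDoor message, passing itself, to the hit actor.
; The key destroys itself when its OnDoorOpened event fires, and the drop event is overridden to do nothing.
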(event EventDropInventory
  (params (DropImpulse :type Vector :default "0, 0, 0") (SpawnTransform :type Transform))
  ;[1 1 1] Cannot Drop Key
)

(event EventUseItem
  (bind _characterowner (Variables|Default|GetCharacterOwner))
  (bind _returnvalue (Transformation|GetActorLocation _characterowner))
  ;[1 1 1] Comment
  (bind _outhit (Collision|LineTraceByChannel _returnvalue (+ (* (Transformation|GetActorForwardVector _characterowner) 200) _returnvalue) "TraceTypeQuery1" false (Utilities|Array|MakeArray (Variables|Default|GetCharacterOwner)) "None"))
  (if (.bBlockingHit (Collision|BreakHitResult _outhit))
    (Class|BPIInteract|TryOpenDoor(Message) (.HitActor (Collision|BreakHitResult _outhit)) self)))

(event EventOnDoorOpened
  ;[1 1 1] On Door Opened
  (Actor|DestroyActor))

(fn ConstructionScript
  (|CallParentFunction))