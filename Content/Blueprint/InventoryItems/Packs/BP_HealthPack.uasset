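; BP_HealthPack is an inventory pack item that heals the character that owns it when used.
; On UseItem it casts CharacterOwner to BP_MGJCharacter, adds AmountToHeal to Health capped at MaxHealth, then destroys itself.
; If the cast fails, nothing happens and the item is not consumed.
; The construction script only calls the parent's.
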(event EventUseItem
  ;[1 1 1] Use item
  (bind _asbp_mgjcharacter (Utilities|Casting|CastToBP_MGJCharacter (Variables|Default|GetCharacterOwner)))
  (Variables|/Game/Blueprint/Player/Character/BP_MGJCharacter.BP_MGJCharacter_C|SetHealth _asbp_mgjcharacter (Math|Float|Min(Float) (+ (Variables|/Game/Blueprint/Player/Character/BP_MGJCharacter.BP_MGJCharacter_C|GetHealth _asbp_mgjcharacter) (Variables|Default|GetAmountToHeal)) (Variables|/Game/Blueprint/Player/Character/BP_MGJCharacter.BP_MGJCharacter_C|GetMaxHealth _asbp_mgjcharacter)))
  (Actor|DestroyActor))

(fn ConstructionScript
  (|CallParentFunction))