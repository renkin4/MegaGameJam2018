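; Base spectacles inventory item that changes global time dilation while keeping the owning character at normal speed through inverse custom time dilation.
; First use starts a self-destruct timer, with its duration scaled by the dilation; later uses resume it.
; The secondary use restores normal time and pauses the timer, preserving the remaining duration.
; Self-destruct restores normal time and destroys the item.
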(event Custom|ReturnToDefault
  ;[1 1 1] Time Dil
  (Utilities|Time|SetGlobalTimeDilation 1.0)
  (Variables|/Script/Engine.Actor|SetCustomTimeDilation (Variables|Default|GetCharacterOwner) 1.0))

(event Custom|SelfDestruct
  ;[1 1 1] Self Destruct
  (CallFunction|ReturntoDefault)
  (Actor|DestroyActor))

(event EventUseItem
  ;[1 1 1] Event Use Item
  (Utilities|Time|SetGlobalTimeDilation (Variables|Default|GetTimeDilVal))
  (Variables|/Script/Engine.Actor|SetCustomTimeDilation (Variables|Default|GetCharacterOwner) (/ 1.0 (Variables|Default|GetTimeDilVal)))
  (if (not (Utilities|Time|IsValidTimerHandle (Variables|Default|GetTimerHandle_SelfDestruct)))
    (bind _returnvalue (Utilities|Time|SetTimerbyEvent (EventDispatchers|CreateEvent :!event Custom|SelfDestruct) (* (Variables|Default|GetSpecDuration) (Class|GameplayStatics|GetGlobalTimeDilation))))
    (Variables|Default|SetTimerHandle_SelfDestruct _returnvalue)
    (else
      (Utilities|Time|UnpauseTimerbyHandle (Variables|Default|GetTimerHandle_SelfDestruct)))))

(event EventUseItem2
  ;[1 1 1] Use item 2
  (if (Utilities|Time|IsValidTimerHandle (Variables|Default|GetTimerHandle_SelfDestruct))
    (CallFunction|ReturntoDefault)
    (Utilities|Time|PauseTimerbyHandle (Variables|Default|GetTimerHandle_SelfDestruct))))

(fn ConstructionScript
  (|CallParentFunction))