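; Base weapon inventory item that fires projectiles from its owning character and tracks clip and reserve ammo.
; Primary use spawns a BP_ProjectileBase ahead of the owner along its facing and decrements the clip, or starts a reload when empty.
; Secondary use reloads manually; both reloads follow a retriggerable delay and move reserve ammo into the clip.
; RefillAmmo tops up the capped reserve, and Tick prints ammo counts for debugging.
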(event Custom|RefillAmmo
  (params (Amount :type Integer))
  ;[1 1 1] Refill Ammo
  (Variables|Default|SetCurrentAmmo (Math|Integer|Min(Integer) (+ (Variables|Default|GetCurrentAmmo) Amount) (Variables|Default|GetMaxAmmo))))

(event EventUseItem2
  ;[1 1 1] Manual Reload
  (Utilities|FlowControl|RetriggerableDelay (Variables|Default|GetReloadDuration))
  (CallFunction|StartReload))

(event EventUseItem
  ;[1 1 1] Shoot Gun
  (Utilities|FlowControl|Sequence
    (:then_0
      (if (> (Variables|Default|GetCurrentAmmoClip) 0)
        (Projectile|SpawnProjectile
          (:then2
            (Math|Integer|DecrementInt (Variables|Default|GetCurrentAmmoClip))))
        (else
          (Utilities|FlowControl|RetriggerableDelay (Variables|Default|GetReloadDuration))
          (CallFunction|StartReload))))))

(event EventTick
  (params (DeltaSeconds :type Float%20%28single-precision%29))
  ;[1 1 1] Event Tick
  (Development|PrintString (Utilities|String|Append (Utilities|String|ToString(Integer) (Variables|Default|GetCurrentAmmoClip)) " ++ " (Utilities|String|ToString(Integer) (Variables|Default|GetCurrentAmmo))) true true "(R=0.000000,G=0.660000,B=1.000000,A=1.000000)" DeltaSeconds))

(fn ConstructionScript
  (|CallParentFunction))

(fn StartReload
  (if (CallFunction|CanReload)
    (LocalVariables|SetClipDelta (Math|Integer|Min(Integer) (- (Variables|Default|GetMaxClipAmmo) (Variables|Default|GetCurrentAmmoClip)) (- (Variables|Default|GetCurrentAmmo) (Variables|Default|GetCurrentAmmoClip))))
    (Utilities|FlowControl|Sequence
      (:then_0
        (if (> (LocalVariables|GetClipDelta) 0)
          (Variables|Default|SetCurrentAmmoClip (+ (Variables|Default|GetCurrentAmmoClip) (LocalVariables|GetClipDelta)))
          (Variables|Default|SetCurrentAmmo (- (Variables|Default|GetCurrentAmmo) (LocalVariables|GetClipDelta))))))))

(fn CanReload
  (return (> (Variables|Default|GetCurrentAmmo) 0)))