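; Player character Blueprint with health, forward movement and a cyclable slot-based inventory; MoveRight input is left unwired.
; On possession it caches the HUD, spawns inventory slot actors, creates the main widget and selects the first slot.
; Inputs use or cycle the current slot with wraparound, and AddToInventory fills it, or another empty slot when occupied.
; Any damage lowers Health, while point damage launches the character opposite the hit normal.
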(event Custom|SetupDefaultInventory
  (bind _self self)
  ;[0 0 1] CreateDefaultInventory
  (Utilities|FlowControl|Sequence
    (:then_0
      (for _index (range 0 3)
        (bind _returnvalue (Game|SpawnActorfromClass "/Game/Blueprint/InventoryItems/BP_InventorySlot.BP_InventorySlot_C" (Math|Transform|MakeTransform "0, 0, 0" "0, 0, 0" "1,1,1") "AlwaysSpawn" 0 _self _self))
        (Utilities|Array|Add (Variables|Inventory|GetCharacterInventory) _returnvalue))
      (Variables|Inventory|SetCurrentInventory (Utilities|Array|Get(acopy) (Variables|Inventory|GetCharacterInventory))))))

(event EventPossessed
  (params (NewController :type Controller%20Object%20Reference))
  ;[0 0.4408 1] Event On possessed
  (Utilities|FlowControl|Sequence
    (:then_0
      (bind _asplayer_controller (Utilities|Casting|CastToPlayerController NewController))
      (bind _asbp_mgjhud (Utilities|Casting|CastToBP_MGJHUD (HUD|GetHUD _asplayer_controller)))
      (Variables|HUD|SetMGJHUD _asbp_mgjhud))
    (:then_1
      (bind _mgjhud (Variables|HUD|GetMGJHUD)
        (:then
          (CallFunction|SetupDefaultInventory)
          (Default|CreateMainWidget _mgjhud)
          (CallFunction|SwitchInventory))
        (:else)))))

(event Game|Damage|EventPointDamage
  (params (Damage :type Float%20%28single-precision%29) (DamageType :type Damage%20Type%20Object%20Reference) (HitLocation :type Vector :default "0, 0, 0") (HitNormal :type Vector :default "0, 0, 0") (HitComponent :type Primitive%20Component%20Object%20Reference) (BoneName :type Name :default "None") (ShotFromDirection :type Vector :default "0, 0, 0") (InstigatedBy :type Controller%20Object%20Reference) (DamageCauser :type Actor%20Object%20Reference) (HitInfo :type Hit%20Result%20Structure%20%28by%20ref%29))
  ;[1 0 0.8394] Damage
  ;;[1 1 1] On Receive Any Point Damage
  (Character|LaunchCharacter (* (* HitNormal -1) 1e+03) true true))

(event Game|Damage|EventAnyDamage
  (params (Damage :type Float%20%28single-precision%29) (DamageType :type Damage%20Type%20Object%20Reference) (InstigatedBy :type Controller%20Object%20Reference) (DamageCauser :type Actor%20Object%20Reference))
  ;[1 0 0.8394] Damage
  ;;[1 1 1] Event Any Damage
  (Variables|Player|SetHealth (Math|Float|Max(Float) (- (Variables|Player|GetHealth) Damage) 0.0)))

(event Input|ActionEvents|InputActionUseCurrentInventory
  (params (Key :type Key%20Structure))
  ;[0 1 0.09764] Inventory Inputs
  (:Pressed
    (bind _currentinventory (Variables|Inventory|GetCurrentInventory)
      (:then
        (Default|UseItem _currentinventory))
      (:else))))

(event Input|ActionEvents|InputActionNextInventory
  (params (Key :type Key%20Structure))
  ;[0 1 0.09764] Inventory Inputs
  (:Pressed
    (CallFunction|SwitchInventory 1)))

(event Input|ActionEvents|InputActionPreviousInventory
  (params (Key :type Key%20Structure))
  ;[0 1 0.09764] Inventory Inputs
  (:Pressed
    (CallFunction|SwitchInventory -1)))

(event Input|ActionEvents|InputActionUseCurrentInventory2
  (params (Key :type Key%20Structure))
  ;[0 1 0.09764] Inventory Inputs
  (:Pressed
    (bind _currentinventory (Variables|Inventory|GetCurrentInventory)
      (:then
        (Default|UseItem2 _currentinventory))
      (:else))))

(event Input|AxisEvents|InputAxisMoveRight
  (params (AxisValue :type Float%20%28single-precision%29))
  ;[1 0.9893 0] Movement Inputs
)

(event Input|AxisEvents|InputAxisMoveForward
  (params (AxisValue :type Float%20%28single-precision%29))
  ;[1 0.9893 0] Movement Inputs
  (Pawn|Input|AddMovementInput (Math|Vector|GetForwardVector (Transformation|GetActorRotation)) AxisValue false))

(fn ConstructionScript)

(fn ChangeCurrentInventory
  (params (NewInventory :type BP%20Inventory%20Slot%20Object%20Reference))
  (LocalVariables|SetPreviousInventory (Variables|Inventory|GetCurrentInventory))
  (Variables|Inventory|SetCurrentInventory NewInventory)
  (Default|OnSelected (Variables|Inventory|GetCurrentInventory))
  (if (!= (Variables|Inventory|GetCurrentInventory) (LocalVariables|GetPreviousInventory))
    (bind _previousinventory (LocalVariables|GetPreviousInventory)
      (:then
        (Default|OnDeSelect _previousinventory))
      (:else))))

(fn SwitchInventory
  (params (NextIndex :type Integer))
  (LocalVariables|Setm_NextIndex (Math|Integer|Clamp(Integer) NextIndex -1 1))
  (LocalVariables|SetCurrentIndex (Utilities|Array|FindItem (Variables|Inventory|GetCharacterInventory) (Variables|Inventory|GetCurrentInventory)))
  (LocalVariables|Setm_NextIndex (Math|Integer|%(Integer) (+ (LocalVariables|GetCurrentIndex) (LocalVariables|Getm_NextIndex)) (Utilities|Array|Length (Variables|Inventory|GetCharacterInventory))))
  (if (< (LocalVariables|Getm_NextIndex) 0)
    (LocalVariables|Setm_NextIndex (Utilities|Array|LastIndex (Variables|Inventory|GetCharacterInventory))))
  (CallFunction|ChangeCurrentInventory (Utilities|Array|Get(acopy) (Variables|Inventory|GetCharacterInventory) (LocalVariables|Getm_NextIndex))))

(fn AddtoInventory
  (params (Inventory :type BP%20Inventory%20Item%20Base%20Object%20Reference))
  (if (Default|IsValidSlot (Variables|Inventory|GetCurrentInventory))
    (bind _array_element (Utilities|Array|ForEachLoopwithBreak (Variables|Inventory|GetCharacterInventory) :!label _label)
      (:LoopBody
        (if (not (Default|IsValidSlot _array_element))
          (LocalVariables|SetSelectedSlot _array_element)
          (goto _label Break)))
      (:Completed
        (bind _selectedslot (LocalVariables|GetSelectedSlot)
          (:then
            (Default|SetInventory _selectedslot Inventory)
            (return true))
          (:else
            (return false)))))
    (else
      (Default|SetInventory (Variables|Inventory|GetCurrentInventory) Inventory)
      (return true))))